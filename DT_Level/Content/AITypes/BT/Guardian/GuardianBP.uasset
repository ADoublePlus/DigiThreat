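; GuardianBP is the guardian AI pawn, driven by a behavior tree.
; On BeginPlay it casts its controller to My_AIC and passes it the behavior tree, with the player pawn as the pawn-sensing target.
; Its construction script creates a dynamic emissive material on the Eye mesh and hands it to a GenericEmissiveColourChanging component, which can then alter the eye colour.
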(event `self.ReceiveBeginPlay`
  ;[1 1 1] Begin play
  (bind _asmy_aic (cast `/Game/AITypes/BT/My_AIC` (`AIBlueprintHelperLibrary.GetAIController` self)))
  (`/Game/AITypes/BT/My_AIC.Setup AIC` _asmy_aic (`self.BT`) (`GameplayStatics.GetPlayerPawn` 0)))

(fn `UserConstructionScript`
  ;[1 1 1] Setup dynamic eye material and component
  (bind _returnvalue (`PrimitiveComponent.CreateDynamicMaterialInstance` (`self.Eye`) 0 "/Game/AITypes/BT/Guardian/GenericEmissiveColour.GenericEmissiveColour" "None"))
  (bind _output_get (set `self.DynamicEyeMatRef` _returnvalue))
  (`/Game/AITypes/BT/Guardian/GenericEmissiveColourChangingComponent.Setup` (`self.GenericEmissiveColourChangingComponent`) _output_get))