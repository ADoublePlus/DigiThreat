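; Skywatcher is a flying AI character with a glowing eye, driven by a behaviour tree.
; On BeginPlay it passes that tree and the player pawn, as the sensing target, to its AI controller.
; Its construction script creates a dynamic eye material for the emissive colour-changing component and initialises the physics move-to parameters.
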(event `self.ReceiveBeginPlay`
  (bind _asmy_aic (cast `` (`AIBlueprintHelperLibrary.GetAIController` self)))
  (`self.Setup AIC` _asmy_aic (`self.BT`) (`GameplayStatics.GetPlayerPawn` 0)))

(fn `UserConstructionScript`
  ;[1 1 1] Setup dynamic eye material and component
  (bind _returnvalue (`PrimitiveComponent.CreateDynamicMaterialInstance` (`self.Eye`) 0 null "None"))
  (bind _output_get (set `self.DynamicEyeMatRef` _returnvalue))
  (`self.Setup` (`self.GenericEmissiveColourChangingComponent`) _output_get)
  ;[1 1 1] Setup physics movement
  (`/Game/FlyingAIType/BT/FlyingAI/PhysicsMoveToParameters.Setup` (`self.PhysicsMoveToParameters`)))