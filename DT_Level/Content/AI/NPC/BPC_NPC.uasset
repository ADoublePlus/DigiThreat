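; Enemy NPC that takes flame damage, plays melee attacks and hurts the player on contact.
; Overlapping FlameProjectile or FlameVortex spawns an explosion and lowers Health, destroying the NPC at zero; only projectile kills increment Player KillCount.
; A mesh-attached sphere damages BP_Rifle_Character and shows a DamageArrow widget, independently of the melee montage.
; AnyDamage sets Health to Damage minus Health and updates the health bar, whose setup logic is disconnected.
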(event `self.ReceiveActorBeginOverlap`
  (params (OtherActor :type "Actor Object Reference"))
  (`|ExecutionSequence`
    (:`then_0`
      (bind _asflame_projectile (cast `/Game/Character/Spell_BP/FlameProjectile` OtherActor))
      (`GameplayStatics.SpawnEmitterAtLocation` "/Game/StarterContent/Particles/P_Explosion.P_Explosion" (`self.K2_GetActorLocation` _asflame_projectile))
      (bind _output_get (set `self.Health` (- (`self.Health`) 0.25)))
      (if (<= _output_get 0.0)
        (`self.K2_DestroyActor` _asflame_projectile)
        (`self.K2_DestroyActor`)
        (bind _asplayer (cast `/Game/Character/Humanoid/Player` (`GameplayStatics.GetPlayerCharacter` 0)))
        (set `/Game/Character/Humanoid/Player.KillCount` (+ (`/Game/Character/Humanoid/Player.KillCount` _asplayer) 1) _asplayer)
        (else
          (`self.K2_DestroyActor` _asflame_projectile))))
    (:`then_1`
      (bind _asflame_vortex (cast `/Game/Character/Spell_BP/FlameVortex` OtherActor))
      (`GameplayStatics.SpawnEmitterAtLocation` "/Game/StarterContent/Particles/P_Explosion.P_Explosion" (`self.K2_GetActorLocation` _asflame_vortex))
      (bind _output_get_2 (set `self.Health` (- (`self.Health`) 0.3)))
      (if (<= _output_get_2 0.0)
        (`self.K2_DestroyActor`)))))

(event `self.ReceiveBeginPlay`)

(event `self.ReceiveAnyDamage`
  (params (Damage :type "Float (single-precision)") (DamageType :type "DamageType Object Reference") (InstigatedBy :type "Controller Object Reference") (DamageCauser :type "Actor Object Reference"))
  (set `self.Health` (- Damage (`self.Health`)))
  (`/Game/AI/NPC/EnemyHealth.UpdateHealth` (`self.AiHealthBarWidget`)))

(event `/Game/AI/NPC/CombatInterface.MeleeAttack`
  (`|PlayMontage` (`self.Mesh`) "/Game/AI/NPC/Attack_PrimaryA_Montage.Attack_PrimaryA_Montage"
    (:`then`
      (`GameplayStatics.PlaySound2D` "/Game/SoundsAndFX/punch_or_whack_-Vladimir-403040765_Cue.punch_or_whack_-Vladimir-403040765_Cue" 1.0 1.0 0.0 null null))))

(event `self.Sphere.OnComponentBeginOverlap`
  (params (OverlappedComponent :type "PrimitiveComponent Object Reference") (OtherActor :type "Actor Object Reference") (OtherComp :type "PrimitiveComponent Object Reference") (OtherBodyIndex :type Integer) (bFromSweep :type Boolean) (SweepResult :type "HitResult Structure (by ref)"))
  (bind _asbp_rifle_character (cast `/Game/FPS_Character_Assets/BP_Rifle_Character` OtherActor))
  (`KismetSystemLibrary.PrintString` "enemy hit")
  (set `/Game/FPS_Character_Assets/BP_Rifle_Character.Health` (- (`/Game/FPS_Character_Assets/BP_Rifle_Character.Health` _asbp_rifle_character) 0.2) _asbp_rifle_character)
  (bind _returnvalue (`|CreateWidget` "/Game/FPS_Character_Assets/Damage_Indicator/Widgets/DamageArrow.DamageArrow_C" (`GameplayStatics.GetPlayerController` 0)))
  (`UserWidget.AddToViewport` _returnvalue 0))

(fn `UserConstructionScript`
  (`SceneComponent.K2_AttachToComponent` (`self.Sphere`) (`self.Mesh`) "None" "KeepRelative" "KeepRelative" "KeepRelative" true))